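; Pressure button platform that glows and shifts down when actors tagged Player step on it.
; At start it creates a dynamic glow material and can pass its color to linked platforms through BPI_EmissionMaterial.
; An overlap counter keeps it lit until the last tagged actor leaves.
; A Timeline lerps the actor's Z from its current height toward an offset above or below the saved starting height.
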(event EventBeginPlay
  ;[1 1 1] Sets Button platform base color to desired value passed and emissiveness to 0
  (bind _returnvalue (Rendering|Material|CreateDynamicMaterialInstance (Rendering|Material|GetMaterial (Variables|Default|GetButtonMesh) 0) "Glow" "None" :!class /Script/Engine.KismetMaterialLibrary))
  (bind _output_get (Variables|Material|SetGlowingDynamicMaterial _returnvalue))
  (Rendering|Material|SetVectorParameterValue _output_get "Base Color" (Variables|TriggerSettings|Material|GetObjectColor) :!class /Script/Engine.MaterialInstanceDynamic)
  (CallFunction|SetEmissiveness 0.0 (Variables|Default|GetButtonMesh) (Variables|Material|GetGlowingDynamicMaterial))
  ;[1 1 1] Save Actor original Z pos for button anim
  (Variables|Useful|SetActorOrginizalZ (.z (Transformation|GetActorLocation)))
  (Utilities|FlowControl|DelayUntilNextTick)
  ;[1 1 1] Sets all platforms that depends of this trigger to have the same color
  (if (Variables|TriggerSettings|Material|GetSetInfluencedPlatfromsColor)
    (for _array_element (Variables|Default|GetPlatformsToTrigger)
      (bind _tested_object (Utilities|DoesObjectImplementInterface "/Game/Blueprints/OtherClasses/Interfaces/BPI_EmissionMaterial.BPI_EmissionMaterial_C" _array_element)
        (:Implements
          (Class|BPIEmissionMaterial|SetEmissionColor(Message) _tested_object (Variables|TriggerSettings|Material|GetObjectColor self)))))))

(event OnComponentBeginOverlap(TriggerVolume)
  (params (OverlappedComponent :type Primitive%20Component%20Object%20Reference) (OtherActor :type Actor%20Object%20Reference) (OtherComp :type Primitive%20Component%20Object%20Reference) (OtherBodyIndex :type Integer) (bFromSweep :type Boolean) (SweepResult :type Hit%20Result%20Structure%20%28by%20ref%29))
  ;[1 1 1] Make Button Platform glow when steping in it
  (if (Actor|ActorHasTag OtherActor "Player")
    (Math|Integer|IncrementInt (Variables|Useful|GetNumberOfThingsOnTopOfButton)
      (:%20%20
        (CallFunction|SetEmissiveness (Variables|ButtonVisualSettings|GetEmissivenessWhenPressed) (Variables|Default|GetButtonMesh) (Variables|Material|GetGlowingDynamicMaterial))
        (CallFunction|MoveButton false)))))

(event OnComponentEndOverlap(TriggerVolume)
  (params (OverlappedComponent :type Primitive%20Component%20Object%20Reference) (OtherActor :type Actor%20Object%20Reference) (OtherComp :type Primitive%20Component%20Object%20Reference) (OtherBodyIndex :type Integer))
  ;[1 1 1] Make Button Platform stop glowing when not steping in it
  (if (Actor|ActorHasTag OtherActor "Player")
    (Variables|Useful|SetNumberOfThingsOnTopOfButton (Math|Integer|Max(Integer) (- (Variables|Useful|GetNumberOfThingsOnTopOfButton) 1)))
    (if (<= (Variables|Useful|GetNumberOfThingsOnTopOfButton) 0)
      (CallFunction|SetEmissiveness 0.0 (Variables|Default|GetButtonMesh) (Variables|Material|GetGlowingDynamicMaterial))
      (CallFunction|MoveButton true))))

(event Custom|MoveButton
  (params (bMoveUp :type Boolean))
  (bind _returnvalue (Transformation|GetActorLocation))
  ;[1 1 1] Moves Button Up or Down to make it looks like its pressed
  (bind _amountofmovement (Timeline|Timeline PlayFromStart)
    (:Update
      (Transformation|SetActorLocation (Math|Vector|MakeVector (.x _returnvalue) (.y _returnvalue) (Math|Float|Lerp (.z _returnvalue) (- (Variables|Useful|GetActorOrginizalZ) (* (select bMoveUp -1.0 1.0) (Variables|ButtonVisualSettings|GetButtonAnimMovementZ))) _amountofmovement)) false false))))

(fn ConstructionScript)