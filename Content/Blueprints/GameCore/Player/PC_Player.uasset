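; Player controller that handles UI input and opens the pause menu.
; On BeginPlay it adds the player UI mapping context to the Enhanced Input subsystem of player 0.
; The pause menu input action calls ShowPauseMenu, which lazily creates and caches the pause widget, then adds it to or removes it from the viewport.
; The input binding only shows the menu; it does not toggle it, pause the game or change input mode.
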(event EventBeginPlay
  ;[1 1 1] Adds InputMapping for UI
  (Input|AddMappingContext (PlayerController|LocalPlayerSubsystems|GetEnhancedInputLocalPlayerSubsystem (Game|GetPlayerController 0)) "/Game/Blueprints/Input/Player/IMC_PlayerUI.IMC_PlayerUI" 0 "(bIgnoreAllPressedKeysUntilRelease=True,bForceImmediately=False,bNotifyUserSettings=False)"))

(event Input|EnhancedActionEvents|EnhancedInputActionIA_PauseMenu
  (params (ActionValue :type Boolean) (ElapsedSeconds :type Float%20%28double-precision%29) (TriggeredSeconds :type Float%20%28double-precision%29) (InputAction :type Input%20Action%20Object%20Reference :default "/Game/Blueprints/Input/Player/InputAction/UI/IA_PauseMenu.IA_PauseMenu"))
  (:Started
    (CallFunction|ShowPauseMenu true)))

(fn ConstructionScript)

(fn ShowPauseMenu
  (params (bShow :type Boolean))
  ;[1 1 1] Show or Hide Pause widget
  (Variables|Default|GetPauseMenu
    (:then
      _)
    (:else
      (bind _returnvalue (UserInterface|CreateWidget "/Game/Blueprints/UI/Widgets/PauseMenu/WB_PauseMenu.WB_PauseMenu_C" self))
      (Variables|Default|SetPauseMenu _returnvalue)))
  (if bShow
    (UserInterface|Viewport|AddtoViewport (Variables|Default|GetPauseMenu) 0)
    (else
      (Widget|RemovefromParent (Variables|Default|GetPauseMenu)))))