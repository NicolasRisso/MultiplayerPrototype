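; Player controller for the main menu that shows the main menu widget on BeginPlay.
; It shows or hides the main menu, create-server and server browser screens through the BPI_HUD_MainMenu interface.
; Widgets are created on first use, cached in a map keyed by screen type, then added to or removed from the viewport.
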(event EventBeginPlay
  ;[1 1 1] Show Widget
  (Widget|Show/HideWidget "NewEnumerator0" true))

(event EventCallShow/HideWidget
  (params (Widget :type E_MainMenuWidgets%20Enum :default "NewEnumerator0") (Show :type Boolean))
  ;[1 1 1] BPI_HUD_MainMenu
  (Widget|Show/HideWidget Widget Show))

(fn ConstructionScript)

(fn ShowWidget
  (params (Widget :type E_MainMenuWidgets%20Enum :default "NewEnumerator0"))
  (Utilities|IsValid (.Value (Utilities|Map|Find (Variables|Widget|GetWidgetMap) Widget))
    (:Is%20Valid
      _)
    (:Is%20Not%20Valid
      (bind _returnvalue (UserInterface|CreateWidget (Utilities|Select :Index Widget :NewEnumerator0 "/Game/Blueprints/UI/Widgets/MainMenu/WB_MainMenu.WB_MainMenu_C" :NewEnumerator1 "/Game/Blueprints/UI/Widgets/MainMenu/WB_CreateServer.WB_CreateServer_C" :NewEnumerator2 "/Game/Blueprints/UI/Widgets/MainMenu/WB_ServerBrowser.WB_ServerBrowser_C")))
      (Utilities|Map|Add (Variables|Widget|GetWidgetMap) Widget _returnvalue)))
  (UserInterface|Viewport|AddtoViewport (.Value (Utilities|Map|Find (Variables|Widget|GetWidgetMap) Widget)) 0))

(fn HideWidget
  (params (Widget :type E_MainMenuWidgets%20Enum :default "NewEnumerator0"))
  (bind _widgetmap (Variables|Widget|GetWidgetMap))
  (bind _value (Utilities|Map|Find _widgetmap Widget))
  (Utilities|IsValid _value
    (:Is%20Valid
      (Widget|RemovefromParent _value))))

(fn Show/HideWidget
  (params (Widget :type E_MainMenuWidgets%20Enum :default "NewEnumerator0") (Show :type Boolean))
  (if Show
    (Widget|ShowWidget Widget)
    (else
      (Widget|HideWidget Widget))))